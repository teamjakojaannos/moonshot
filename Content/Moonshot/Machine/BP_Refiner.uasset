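; Refinery machine that takes deposited rock and turns it into refined ore.
; The construction script registers it as the deposit target of its child deposit trigger through BPI_DepositTarget.
; Accept rejects deposits at full capacity, otherwise increments the rock count and starts a looping timer if none is running.
; Each tick spawns RefineryYield ore actors at OreOutput, consumes one rock and clears the timer once empty.
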(event `StartProcessing`
  (params (Depositable :type "/Game/Moonshot/Loot/BPI_Depositable Interface"))
  (if (not (`KismetSystemLibrary.K2_IsValidTimerHandle` (`self.ProcessTimer`)))
    (bind _returnvalue (`KismetSystemLibrary.K2_SetTimerDelegate` (delegate `ProcessingTick`) (`self.ProcessingTime`) true))
    (set `self.ProcessTimer` _returnvalue)))

(event `ProcessingTick`
  (for _ (range 1 (+ (`self.RefineryYield`) 1))
    (`|SpawnActorFromClass` "/Game/Moonshot/Loot/BP_Refined_Ore.BP_Refined_Ore_C" (`SceneComponent.K2_GetComponentToWorld` (`self.OreOutput`)) "Undefined" "OverrideRootScale" null null))
  (`self.UpdateInventory`)
  (if (<= (`self.InventoryRockAmount`) 0)
    (`KismetSystemLibrary.K2_ClearAndInvalidateTimerHandle` (`self.ProcessTimer`))))

(fn `Accept`
  (params (Depositable :type "/Game/Moonshot/Loot/BPI_Depositable Interface"))
  (returns (bSuccess :type Boolean))
  (bind _inventoryrockamount (`self.InventoryRockAmount`))
  (`/Engine/EditorBlueprintResources/StandardMacros.CompareInt` _inventoryrockamount (`self.InventoryMaxCapacity`)
    (:`>`
      _)
    (:`==`
      _)
    (:`<`
      (`/Engine/EditorBlueprintResources/StandardMacros.IncrementInt` _inventoryrockamount
        (:`  `
          (`self.StartProcessing` Depositable)
          (return true)))))
  (return false))

(fn `UpdateInventory`
  (returns (Result :type Integer))
  (bind _result (`/Engine/EditorBlueprintResources/StandardMacros.DecrementInt` (`self.InventoryRockAmount`))
    (:`  `
      (return _result))))

(fn `UserConstructionScript`
  (bind _asbpi_deposit_target (cast `/Game/Moonshot/Machine/BPI_DepositTarget` self))
  (bind _asbp_deposit_trigger (cast `/Game/Moonshot/Machine/BP_DepositTrigger` (`ChildActorComponent.ChildActor` (`self.Deposit`))))
  (set `/Game/Moonshot/Machine/BP_DepositTrigger.DepositTarget` _asbpi_deposit_target _asbp_deposit_trigger))