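; BP_AnchorSpot is an attachment point that holds a single anchored object at its Sphere.
; AnchorTo snaps the object to the Sphere unless the spot is already occupied, and DetachAnchored releases it and re-enables physics on its root.
; The construction script checks the parent actor for BPI_AnchorHooks, which then receives anchor and detach notifications.
; A validity check clears the occupied flag if the anchored actor becomes invalid.
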(fn `AnchorTo`
  (params (Anchorable :type "Actor Object Reference"))
  (returns (AnchorSuccess :type Boolean))
  (bind _hasanchored (`self.Has Valid Anchored Actor`))
  (if _hasanchored
    (`KismetSystemLibrary.PrintString` "Target obstructed.")
    (return false)
    (else
      (`self.K2_AttachToComponent` Anchorable (`self.Sphere`) "None" "SnapToTarget" "SnapToTarget" "KeepRelative" true)
      (set `self.bHasAnchoredActor` true)
      (set `self.AnchoredActor` Anchorable)
      (if (`self.bParentHasHooks`)
        (`/Game/Moonshot/Machine/BPI_AnchorHooks.OnAnchored` (`self.Hooks`)))
      (return true))))

(fn `DetachAnchored`
  (bind _rootcomponent (`Actor.RootComponent` (`self.AnchoredActor`)))
  (bind _hasanchored (`self.Has Valid Anchored Actor`))
  (if _hasanchored
    (`SceneComponent.K2_DetachFromComponent` _rootcomponent "KeepWorld" "KeepWorld" "KeepRelative" true)
    (set `self.bHasAnchoredActor` false)
    (bind _asprimitive_component (cast `PrimitiveComponent` _rootcomponent)
      (:`then`
        (`PrimitiveComponent.SetSimulatePhysics` _asprimitive_component true))
      (:`CastFailed`
        (`KismetSystemLibrary.PrintString` "Failed to cast to primitive component!" true true (struct :`R` 1.0 :`A` 1.0))))
    (if (`self.bParentHasHooks`)
      (`/Game/Moonshot/Machine/BPI_AnchorHooks.OnDetach` (`self.Hooks`)))
    (return)))

(fn `Has Valid Anchored Actor`
  (returns (HasAnchored :type Boolean))
  (if (`self.bHasAnchoredActor`)
    (if (`KismetSystemLibrary.IsValid` (`self.AnchoredActor`))
      (return true)
      (else
        (set `self.bHasAnchoredActor` false))))
  (return false))

(fn `UserConstructionScript`
  (bind _asbpi_anchor_hooks (cast `/Game/Moonshot/Machine/BPI_AnchorHooks` (`self.GetParentActor` (`ActorComponent.GetOwner` (`self.Sphere`))))
    (:`then`
      (set `self.Hooks` _asbpi_anchor_hooks)
      (set `self.bParentHasHooks` true))
    (:`CastFailed`
      (set `self.bParentHasHooks` false))))