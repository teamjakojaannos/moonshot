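; BP_ButtonGoHome is an interactable button that checks whether the team has met the ore quota to win the game.
; Interact runs its check only on the server, comparing DepositedOreAmount with RequiredOreAmount on BP_MoonshotGameState.
; The result is only a printed win, get-back-to-work or cast-error message; no actual end-of-game logic runs here.
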(fn `Interact`
  (if (`KismetSystemLibrary.IsServer`)
    (bind _asbp_moonshot_game_state (cast `/Game/Moonshot/BP_MoonshotGameState` (`GameplayStatics.GetGameState`))
      (:`then`
        (if (>= (`/Game/Moonshot/BP_MoonshotGameState.DepositedOreAmount` _asbp_moonshot_game_state) (`/Game/Moonshot/BP_MoonshotGameState.RequiredOreAmount` _asbp_moonshot_game_state))
          (`KismetSystemLibrary.PrintString` "You win the game!")
          (return)
          (else
            (`KismetSystemLibrary.PrintString` "Get back to work")
            (return))))
      (:`CastFailed`
        (`KismetSystemLibrary.PrintString` "Error: Failed to cast game state!")
        (return)))
    (else
      (return))))

(fn `UserConstructionScript`)