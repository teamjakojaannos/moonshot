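; Deposit trigger for a machine that feeds overlapping depositable actors into its DepositTarget.
; Actors implementing BPI_Depositable are asked if they fit the target, then offered to it via Accept.
; Success destroys the actor; refusal by either side only prints a fail message.
; Enable and disable events toggle DepositEnabled and the point light color, also set on construction, but the overlap path never checks that flag.
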(event `self.ReceiveActorBeginOverlap`
  (params (OtherActor :type "Actor Object Reference"))
  (bind _asbpi_depositable (cast `/Game/Moonshot/Loot/BPI_Depositable` OtherActor))
  (`self.DepositableBeginOverlap` _asbpi_depositable OtherActor))

(event `DepositableBeginOverlap`
  (params (AsDepositable :type "/Game/Moonshot/Loot/BPI_Depositable Interface") (Actor :type "Actor Object Reference"))
  (bind _bcanbedeposited (`/Game/Moonshot/Loot/BPI_Depositable.CanBeDepositedInto` AsDepositable (`self.DepositTarget`)))
  (if _bcanbedeposited
    (bind _bsuccess (`/Game/Moonshot/Machine/BPI_DepositTarget.Accept` (`self.DepositTarget`) AsDepositable))
    (if _bsuccess
      (`self.DepositSuccess` AsDepositable Actor)
      (else
        (`self.DepositFail` AsDepositable Actor :!label _label)))
    (else
      (goto _label))))

(event `DepositSuccess`
  (params (AsDepositable :type "/Game/Moonshot/Loot/BPI_Depositable Interface") (Actor :type "Actor Object Reference"))
  (`self.K2_DestroyActor` Actor))

(event `DepositFail`
  (params (AsDepositable :type "/Game/Moonshot/Loot/BPI_Depositable Interface") (Actor :type "Actor Object Reference"))
  (`KismetSystemLibrary.PrintString` "Deposit fail"))

(event `EnableDeposit`
  (if (not (`self.bDepositEnabled`))
    (set `self.bDepositEnabled` true)
    (`LightComponent.SetLightColor` (`self.PointLight`) (`self.EnabledColor`) true)))

(event `DisableDeposit`
  (if (`self.bDepositEnabled`)
    (set `self.bDepositEnabled` false)
    (`LightComponent.SetLightColor` (`self.PointLight`) (`self.DisabledColor`) true)))

(fn `UserConstructionScript`
  (`LightComponent.SetLightColor` (`self.PointLight`) (select `bool` (`self.bDepositEnabled`) :`false` (`self.DisabledColor`) :`true` (`self.EnabledColor`)) true))