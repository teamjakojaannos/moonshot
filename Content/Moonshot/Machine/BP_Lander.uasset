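; Lander machine that serves as a deposit target, keeping a count of rocks deposited into it.
; The construction script registers the lander, through BPI_DepositTarget, as the target of its four child-actor deposit triggers.
; Accept takes any depositable unconditionally and increments RockCount.
; On BeginPlay it hands itself to the WBP_InventoryCounter in its widget component.
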(event `self.ReceiveBeginPlay`
  (bind _aswbp_inventory_counter (cast `/Game/Moonshot/Machine/WBP_InventoryCounter` (`WidgetComponent.GetUserWidgetObject` (`self.InventoryCounter`))))
  (set `/Game/Moonshot/Machine/WBP_InventoryCounter.Lander` self _aswbp_inventory_counter))

(fn `Accept`
  (params (Depositable :type "/Game/Moonshot/Loot/BPI_Depositable Interface"))
  (returns (bSuccess :type Boolean))
  (`/Engine/EditorBlueprintResources/StandardMacros.IncrementInt` (`self.RockCount`)
    (:`  `
      (return true))))

(fn `UserConstructionScript`
  (bind _asbpi_deposit_target (cast `/Game/Moonshot/Machine/BPI_DepositTarget` self))
  (`|ExecutionSequence`
    (:`then_0`
      (bind _asbp_deposit_trigger (cast `/Game/Moonshot/Machine/BP_DepositTrigger` (`ChildActorComponent.ChildActor` (`self.Deposit_1`))))
      (set `/Game/Moonshot/Machine/BP_DepositTrigger.DepositTarget` _asbpi_deposit_target _asbp_deposit_trigger))
    (:`then_1`
      (bind _asbp_deposit_trigger_2 (cast `/Game/Moonshot/Machine/BP_DepositTrigger` (`ChildActorComponent.ChildActor` (`self.Deposit_2`))))
      (set `/Game/Moonshot/Machine/BP_DepositTrigger.DepositTarget` _asbpi_deposit_target _asbp_deposit_trigger_2))
    (:`then_2`
      (bind _asbp_deposit_trigger_3 (cast `/Game/Moonshot/Machine/BP_DepositTrigger` (`ChildActorComponent.ChildActor` (`self.Deposit_3`))))
      (set `/Game/Moonshot/Machine/BP_DepositTrigger.DepositTarget` _asbpi_deposit_target _asbp_deposit_trigger_3))
    (:`then_3`
      (bind _asbp_deposit_trigger_4 (cast `/Game/Moonshot/Machine/BP_DepositTrigger` (`ChildActorComponent.ChildActor` (`self.Deposit_4`))))
      (set `/Game/Moonshot/Machine/BP_DepositTrigger.DepositTarget` _asbpi_deposit_target _asbp_deposit_trigger_4))))