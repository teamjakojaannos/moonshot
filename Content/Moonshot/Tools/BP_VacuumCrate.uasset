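; Grabbable vacuum crate that absorbs overlapping BPI_Storable actors on the server, storing only their classes up to a capacity and destroying them.
; Damage or excessive physics speed spills a random item with an impulse, throttled by a cooldown timer that grabbing also starts.
; It can anchor to an overlapping BP_AnchorSpot (nearest search is a first-result stub) and detaches when grabbed.
; A widget display receives a crate reference.
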(event `self.ReceiveBeginPlay`
  (bind _aswbp_vacuum_crate_display (cast `/Game/Moonshot/Tools/WBP_VacuumCrateDisplay` (`WidgetComponent.GetUserWidgetObject` (`self.Widget`))))
  (set `/Game/Moonshot/Tools/WBP_VacuumCrateDisplay.VacuumCrate` self _aswbp_vacuum_crate_display))

(event `self.ReceiveAnyDamage`
  (params (Damage :type "Float (single-precision)") (DamageType :type "DamageType Object Reference") (InstigatedBy :type "Controller Object Reference") (DamageCauser :type "Actor Object Reference"))
  (if (not (`KismetSystemLibrary.K2_IsValidTimerHandle` (`self.EventTimer`)))
    (`self.SpillContents`)
    (`self.StartSpillCooldown` 2.0)))

(event `EnableAcceptingItems`
  (set `self.bIsAcceptingItems` true))

(event `SpillCooldownTimer`
  (`KismetSystemLibrary.K2_ClearAndInvalidateTimerHandle` (`self.EventTimer`)))

(event `self.ReceiveTick`
  (params (DeltaSeconds :type "Float (single-precision)"))
  (if (`KismetSystemLibrary.IsServer`)
    (if (not (`KismetSystemLibrary.K2_IsValidTimerHandle` (`self.EventTimer`)))
      (bind _returnvalue (`PrimitiveComponent.GetPhysicsLinearVelocity` (`self.Cube`) "None"))
      (if (>= (`KismetMathLibrary.VSizeSquared` _returnvalue) (`KismetMathLibrary.Square` (`self.MaxSpeed`)))
        (`self.SpillContents`)
        (`self.StartSpillCooldown` (`self.SpillCooldown`))))
    (else
      (`KismetSystemLibrary.Delay` 0.6))))

(event `self.ReceiveActorBeginOverlap`
  (params (OtherActor :type "Actor Object Reference"))
  (if (`KismetSystemLibrary.IsServer`)
    (`self.AddActorToStorage` OtherActor)))

(event `/Game/Moonshot/BPI_Interactable.Interact`
  (params (Interactor :type "Actor Object Reference") (HitInfo :type "HitResult Structure"))
  (bind _asbp_player_character (cast `/Game/Moonshot/Characters/BP_PlayerCharacter` Interactor))
  (`self.StartSpillCooldown` 0.2)
  (if (`self.bIsAnchored`)
    (`self.DetachFromAnchorSpot`))
  (`/Game/Moonshot/Characters/BP_PlayerCharacter.GrabByComponent` _asbp_player_character (`self.Cube`) (`SceneComponent.K2_GetComponentRotation` (`MoonshotCharacter.FirstPersonCameraComponent` _asbp_player_character)) (`self.GrabPoint`)))

(event `/Game/Moonshot/Loot/BPI_Breakable.Break`
  (params (NewParam :type Boolean))
  (bind _returnvalue_location (`KismetMathLibrary.BreakTransform` (`SceneComponent.K2_GetComponentToWorld` (`self.Cube`))))
  ;[1 1 1] Soon-to-be redundant
  (`KismetSystemLibrary.PrintString` (`KismetStringLibrary.Concat_StrStr` "There are " (`KismetStringLibrary.Conv_IntToString` (`KismetArrayLibrary.Array_Length` (`self.StoredItems`))) " items inside."))
  (set `self.bIsAcceptingItems` false)
  (for _array_element (`self.StoredItems`)
    (`|SpawnActorFromClass` _array_element (`KismetMathLibrary.MakeTransform` _returnvalue_location) "Undefined" "OverrideRootScale" null null))
  (`KismetArrayLibrary.Array_Clear` (`self.StoredItems`))
  (`self.K2_DestroyActor`))

(event `/Game/Moonshot/Machine/BPI_Anchorable.TryToAnchor`
  (bind _overlappingactors (`PrimitiveComponent.GetOverlappingActors` (`self.AnchorFinder`) "/Game/Moonshot/Machine/BP_AnchorSpot.BP_AnchorSpot_C"))
  (`KismetSystemLibrary.PrintString` "Looking for anchor spots...")
  (if (== (`KismetArrayLibrary.Array_Length` _overlappingactors) 0)
    (`KismetSystemLibrary.PrintString` "No anchors found")
    (else
      (bind _nearest (`self.FindNearestAnchor` _overlappingactors))
      (if (`KismetSystemLibrary.IsValid` _nearest)
        (bind _anchorsuccess (`/Game/Moonshot/Machine/BP_AnchorSpot.AnchorTo` _nearest self))
        (bind _output_get (set `self.bIsAnchored` _anchorsuccess))
        (if _output_get
          (set `self.AnchorSpot` _nearest)
          (`KismetSystemLibrary.PrintString` "Anchoring success!")
          (else
            (`KismetSystemLibrary.PrintString` "Anchoring failed!")))
        (else
          (`KismetSystemLibrary.PrintString` "Non valid anchor spot returned!" true true (struct :`R` 1.0 :`A` 1.0) 4.0))))))

(fn `AddActorToStorage`
  (params (Item :type "Actor Object Reference"))
  (returns (StoreSuccess :type Boolean))
  (if (and (and (`self.bIsAcceptingItems`) (< (`KismetArrayLibrary.Array_Length` (`self.StoredItems`)) (`self.StorageCapacity`))) (`KismetSystemLibrary.DoesImplementInterface` Item "/Game/Moonshot/Tools/BPI_Storable.BPI_Storable_C"))
    (`KismetArrayLibrary.Array_Add` (`self.StoredItems`) (`GameplayStatics.GetObjectClass` Item))
    (`self.K2_DestroyActor` Item)
    (return true)
    (else
      (return false))))

(fn `DetachFromAnchorSpot`
  (bind _anchorspot (`self.AnchorSpot`))
  (set `self.bIsAnchored` false)
  (if (`KismetSystemLibrary.IsValid` _anchorspot)
    (`/Game/Moonshot/Machine/BP_AnchorSpot.DetachAnchored` _anchorspot))
  (return))

(fn `FindNearestAnchor`
  (params (Anchors :type "Array of Actor Object Reference"))
  (returns (Nearest :type "/Game/Moonshot/Machine/BP_AnchorSpot Object Reference"))
  ;[1 1 1] TODO:
  (bind _asbp_anchor_spot (cast `/Game/Moonshot/Machine/BP_AnchorSpot` (`|GetArrayItem` Anchors))
    (:`then`
      (return _asbp_anchor_spot))
    (:`CastFailed`
      (`KismetSystemLibrary.PrintString` "Error converting to BP_AnchorSpot!" true true (struct :`R` 1.0 :`A` 1.0) 4.0))))

(fn `GetItems`
  (returns (Items :type "Array of Actor Class Reference"))
  (return (`self.StoredItems`)))

(fn `GetStoredItemsAmount`
  (returns (Amount :type Integer))
  (return (`KismetArrayLibrary.Array_Length` (`self.StoredItems`))))

(fn `RemoveItemAtIndex`
  (params (Index :type Integer))
  (returns (Item :type "Actor Class Reference"))
  (locals (Temp :type "Actor Class Reference"))
  (bind _storeditems (`self.StoredItems`))
  (bind _output_get (set `local.Temp` (`|GetArrayItem` _storeditems Index)))
  (`KismetArrayLibrary.Array_Remove` _storeditems Index)
  (return _output_get))

(fn `SpillContents`
  (bind _returnvalue (`KismetArrayLibrary.Array_Length` (`self.StoredItems`)))
  (bind (_returnvalue_x _returnvalue_y) (`KismetMathLibrary.BreakVector` (* (`KismetMathLibrary.RandomUnitVector`) 100.0)))
  (bind _returnvalue_2 (`KismetMathLibrary.RandomIntegerInRange` 0 (- _returnvalue 1)))
  (`KismetSystemLibrary.PrintString` "Be careful!")
  (if (> _returnvalue 0)
    (set `self.bIsAcceptingItems` false)
    (`KismetSystemLibrary.K2_SetTimerDelegate` (`|CreateDelegate` :!event `EnableAcceptingItems`) 0.5)
    (bind _returnvalue_3 (`|SpawnActorFromClass` (`|GetArrayItem` (`self.StoredItems`) _returnvalue_2) (`KismetMathLibrary.MakeTransform` (+ (`SceneComponent.K2_GetComponentLocation` (`self.Cube`)) (`KismetMathLibrary.MakeVector` _returnvalue_x _returnvalue_y 50.0)) (`KismetMathLibrary.RandomRotator` true)) "Undefined" "OverrideRootScale" null null))
    (`KismetArrayLibrary.Array_Remove` (`self.StoredItems`) _returnvalue_2)
    (bind _rootcomponent (`Actor.RootComponent` _returnvalue_3))
    (bind _asprimitive_component (cast `PrimitiveComponent` _rootcomponent))
    (bind (_returnvalue_x_2 _returnvalue_y_2) (`KismetMathLibrary.BreakVector` (* (- (`SceneComponent.K2_GetComponentLocation` _rootcomponent) (`SceneComponent.K2_GetComponentLocation` (`self.Cube`))) 2.0)))
    (`PrimitiveComponent.AddImpulse` _asprimitive_component (`KismetMathLibrary.MakeVector` _returnvalue_x_2 _returnvalue_y_2) "None" true)))

(fn `UserConstructionScript`)