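; Assault rifle weapon Blueprint that fires hitscan shots from the owner's eyes, with damage and cosmetic feedback handled separately.
; FireWeapon line traces on the Camera channel out to MaxRange and applies point damage to the hit actor.
; FireWeaponClient skips dedicated servers and, if FireSound is valid, plays it, repeats the trace and spawns a muzzle-to-impact effect actor, tinted red for BP_Alien hits and grey otherwise.
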(event `self.FireWeapon_Client`
  (bind _ownereyes (`self.OwnerEyes`))
  (bind _firesound (`self.FireSound`))
  (bind _returnvalue (`SceneComponent.K2_GetComponentLocation` _ownereyes))
  (bind _returnvalue_2 (`SceneComponent.K2_GetComponentLocation` (`self.MuzzleLocation`)))
  (bind _returnvalue_3 (`SceneComponent.GetForwardVector` _ownereyes))
  (if (not (`KismetSystemLibrary.IsDedicatedServer`))
    (`/Engine/EditorBlueprintResources/StandardMacros.IsValid` _firesound
      (:`Is Valid`
        (`GameplayStatics.PlaySoundAtLocation` _firesound (`self.K2_GetActorLocation`) (struct) 1.0 1.0 0.0 null null null)
        (bind (_outhit _returnvalue_4) (`KismetSystemLibrary.LineTraceSingle` _returnvalue (+ _returnvalue (* (`SceneComponent.GetForwardVector` _ownereyes) (`self.MaxRange`))) "TraceTypeQuery2" true (`|MakeArray` (`ActorComponent.GetOwner` _ownereyes))))
        (`|SpawnActorFromClass` "/Game/Moonshot/BP_BulletTrail.BP_BulletTrail_C" (`KismetMathLibrary.MakeTransform` _returnvalue_2 (`SceneComponent.K2_GetComponentRotation` _ownereyes)) "AlwaysSpawn" "OverrideRootScale" null (select `bool` _returnvalue_4 :`false` (+ _returnvalue_2 (* _returnvalue_3 (`self.MaxRange`))) :`true` (`.ImpactPoint` (`GameplayStatics.BreakHitResult` _outhit))) (select `bool` _returnvalue_4 :`false` (`KismetMathLibrary.NegateVector` _returnvalue_3) :`true` (`.ImpactNormal` (`GameplayStatics.BreakHitResult` _outhit))) (select `bool` (== (`GameplayStatics.GetObjectClass` (`.HitActor` (`GameplayStatics.BreakHitResult` _outhit))) "/Game/Moonshot/Characters/Alien/BP_Alien.BP_Alien_C") :`false` (struct :`R` 0.369792 :`G` 0.369792 :`B` 0.369792 :`A` 1.0) :`true` (struct :`R` 0.359375 :`A` 1.0) :!type "LinearColor Structure") null)))))

(fn `FireWeapon`
  (returns (bShouldFire :type Boolean))
  (bind _ownereyes (`self.OwnerEyes`))
  (bind _returnvalue (`SceneComponent.K2_GetComponentLocation` _ownereyes))
  (bind (_outhit _returnvalue_2) (`KismetSystemLibrary.LineTraceSingle` _returnvalue (+ _returnvalue (* (`SceneComponent.GetForwardVector` _ownereyes) (`self.MaxRange`))) "TraceTypeQuery2" true (`|MakeArray` (`ActorComponent.GetOwner` (`self.OwnerEyes`)))))
  (if _returnvalue_2
    (`GameplayStatics.ApplyPointDamage` (`.HitActor` (`GameplayStatics.BreakHitResult` _outhit)) 20.0 (`SceneComponent.GetForwardVector` (`self.OwnerEyes`)) _outhit (`self.DamageInstigator`) self))
  (return true))

(fn `UserConstructionScript`)