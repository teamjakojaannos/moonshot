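; Lobby trigger actor that starts the mission once every player in a multiplayer game is standing inside it, and destroys itself in standalone play.
; On the server, TriggerArea overlaps maintain a list of lobby characters and refresh the ready count against the game mode's player count.
; When all are ready, it calls StartMission on BP_LobbyGameMode.
; An in-world start-mission widget receives the actor as its target.
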(event `self.ReceiveBeginPlay`
  ;[1 1 1] Destroy self if offline
  (if (`KismetSystemLibrary.IsStandalone`)
    (`self.K2_DestroyActor`)
    (else
      ;[1 1 1] Set up the in-world UI
      (bind _aswbp_start_mission_in_world_ui (cast `/Game/Moonshot/Lobby/WBP_StartMissionInWorldUI` (`WidgetComponent.GetUserWidgetObject` (`self.Widget`))))
      (set `/Game/Moonshot/Lobby/WBP_StartMissionInWorldUI.Target` self _aswbp_start_mission_in_world_ui))))

(event `RefreshReadyCount`
  (bind _returnvalue (`GameplayStatics.GetGameMode`))
  (`/Engine/EditorBlueprintResources/StandardMacros.IsValid` _returnvalue
    (:`Is Valid`
      (bind _returnvalue_2 (`GameModeBase.GetNumPlayers` _returnvalue))
      (set `self.NumPlayers` _returnvalue_2)
      (set `self.NumReady` (`KismetArrayLibrary.Array_Length` (`self.OverlappingPlayers`)))
      (`self.AllPlayersReady`
        (:`true`
          (bind _asbp_lobby_game_mode (cast `/Game/Moonshot/Lobby/BP_LobbyGameMode` (`GameplayStatics.GetGameMode`)))
          (`KismetSystemLibrary.PrintString` "Starting mission!")
          (`MoonshotGameMode.StartMission` _asbp_lobby_game_mode))))))

(event `self.TriggerArea.OnComponentBeginOverlap`
  (params (OverlappedComponent :type "PrimitiveComponent Object Reference") (OtherActor :type "Actor Object Reference") (OtherComp :type "PrimitiveComponent Object Reference") (OtherBodyIndex :type Integer) (bFromSweep :type Boolean) (SweepResult :type "HitResult Structure (by ref)"))
  (if (`KismetSystemLibrary.IsServer`)
    (bind _asbp_lobby_player_character (cast `/Game/Moonshot/Lobby/BP_LobbyPlayerCharacter` OtherActor))
    (`KismetArrayLibrary.Array_AddUnique` (`self.OverlappingPlayers`) _asbp_lobby_player_character)
    (`self.RefreshReadyCount`)))

(event `self.TriggerArea.OnComponentEndOverlap`
  (params (OverlappedComponent :type "PrimitiveComponent Object Reference") (OtherActor :type "Actor Object Reference") (OtherComp :type "PrimitiveComponent Object Reference") (OtherBodyIndex :type Integer))
  (if (`KismetSystemLibrary.IsServer`)
    (bind _asbp_lobby_player_character (cast `/Game/Moonshot/Lobby/BP_LobbyPlayerCharacter` OtherActor))
    (`KismetArrayLibrary.Array_RemoveItem` (`self.OverlappingPlayers`) _asbp_lobby_player_character)
    (`self.RefreshReadyCount`)))

(fn `UserConstructionScript`)