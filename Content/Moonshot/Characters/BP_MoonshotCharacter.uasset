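; BP_MoonshotCharacter is a character Blueprint with basic health, damage and death handling.
; The construction script sets Health to MaxHealth, and AnyDamage subtracts incoming damage, clamped between zero and that maximum.
; At zero health, Death calls OnDeath, an event with no logic here, then destroys the actor.
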(event `self.ReceiveAnyDamage`
  (params (Damage :type "Float (single-precision)") (DamageType :type "DamageType Object Reference") (InstigatedBy :type "Controller Object Reference") (DamageCauser :type "Actor Object Reference"))
  (bind _output_get (set `self.Health` (`KismetMathLibrary.FClamp` (- (`self.Health`) Damage) 0.0 (`self.MaxHealth`))))
  (if (<= _output_get 0.0)
    (`self.Death`)))

(event `Death`
  (`self.OnDeath`)
  (`self.K2_DestroyActor`))

(event `OnDeath`)

(fn `UserConstructionScript`
  (set `self.Health` (`self.MaxHealth`)))