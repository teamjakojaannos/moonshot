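; BP_Alien is an alien character Blueprint that provides a forward hitscan attack.
; Its Attack event traces a line on the Camera channel from the actor's location along its forward vector for AttackRange, with timed debug drawing enabled.
; On a hit, it applies AttackDamage as point damage to the hit actor, crediting its controller as instigator and itself as causer.
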(event `Attack`
  (bind _returnvalue (`self.K2_GetActorLocation`))
  (bind (_outhit _returnvalue_2) (`KismetSystemLibrary.LineTraceSingle` :`Start` _returnvalue :`End` (+ _returnvalue (* (`self.GetActorForwardVector`) (`self.AttackRange`))) :`TraceChannel` "TraceTypeQuery2" :`DrawDebugType` "ForDuration"))
  (if _returnvalue_2
    (`GameplayStatics.ApplyPointDamage` (`.HitActor` (`GameplayStatics.BreakHitResult` _outhit)) (`self.AttackDamage`) (`KismetMathLibrary.NegateVector` (`self.GetActorForwardVector`)) _outhit (`self.GetController`) self)))

(fn `UserConstructionScript`)