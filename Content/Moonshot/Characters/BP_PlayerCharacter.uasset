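; First-person player character for Moonshot that can mine breakable actors and pick up, carry and drop objects.
; Mining and pickup each line-trace forward from the camera: mining calls Break through BPI_Breakable, while pickup attaches the hit component to a physics handle.
; On the server, Tick moves the handle target to GrabNode and clears the holding flag if the grabbed component becomes invalid.
; Debug trace drawing and print messages remain enabled.
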(event `Mine`
  (bind _firstpersoncameracomponent (`self.FirstPersonCameraComponent`))
  (bind _returnvalue (`SceneComponent.K2_GetComponentLocation` _firstpersoncameracomponent))
  (bind (_outhit _returnvalue_2) (`KismetSystemLibrary.LineTraceSingle` :`Start` _returnvalue :`End` (+ _returnvalue (* (`SceneComponent.GetForwardVector` _firstpersoncameracomponent) 500.0)) :`TraceChannel` "TraceTypeQuery1" :`DrawDebugType` "ForDuration" :`DrawTime` 2.0))
  (if _returnvalue_2
    (bind _asbpi_breakable (cast `/Game/Moonshot/Loot/BPI_Breakable` (`.HitActor` (`GameplayStatics.BreakHitResult` _outhit))))
    (`/Game/Moonshot/Loot/BPI_Breakable.Break` _asbpi_breakable false)))

(event `self.ReceiveTick`
  (params (DeltaSeconds :type "Float (single-precision)"))
  (bind _grabhandle (`self.GrabHandle`))
  (if (`KismetSystemLibrary.IsServer`)
    (`PhysicsHandleComponent.SetTargetLocation` _grabhandle (`SceneComponent.K2_GetComponentLocation` (`self.GrabNode`)))
    (set `self.bIsHoldingObject` (and (`KismetSystemLibrary.IsValid` (`PhysicsHandleComponent.GetGrabbedComponent` _grabhandle)) (`self.bIsHoldingObject`)))))

(event `PickObject`
  (bind _firstpersoncameracomponent (`self.FirstPersonCameraComponent`))
  (bind _returnvalue (`SceneComponent.K2_GetComponentLocation` _firstpersoncameracomponent))
  (bind (_outhit _returnvalue_2) (`KismetSystemLibrary.LineTraceSingle` :`Start` _returnvalue :`End` (+ _returnvalue (* (`SceneComponent.GetForwardVector` _firstpersoncameracomponent) (`self.PickupRange`))) :`TraceChannel` "TraceTypeQuery1" :`DrawDebugType` "ForDuration"))
  (if _returnvalue_2
    (bind (_bblockinghit _binitialoverlap _time _distance _location _impactpoint _normal _impactnormal _physmat _hitactor _hitcomponent) (`GameplayStatics.BreakHitResult` _outhit))
    (`PhysicsHandleComponent.GrabComponentAtLocation` (`self.GrabHandle`) _hitcomponent "None" _impactpoint)
    (set `self.bIsHoldingObject` true)
    (`KismetSystemLibrary.PrintString` "Grabbed!")
    (else
      (`KismetSystemLibrary.PrintString` "Nothing to grab."))))

(event `DropObject`
  (`PhysicsHandleComponent.ReleaseComponent` (`self.GrabHandle`))
  (set `self.bIsHoldingObject` false)
  (`KismetSystemLibrary.PrintString` "Dropped!"))

(fn `UserConstructionScript`)