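; BP_OreSpawner is an actor that scatters mineable rocks around its location when play begins.
; It makes Count attempts, each picking a random navigable point within Radius and spawning a BP_Mineable_Rock there with an offset, adjusted for collisions but always spawned.
; Failed navigation queries are skipped without retry, so fewer rocks can appear.
; The random yaw spans only zero to one degree, leaving rocks almost identically oriented.
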(event `self.ReceiveBeginPlay`
  (`self.SpawnOres`))

(event `SpawnOres`
  (for _ (range 1 (+ (`self.Count`) 1))
    (bind (_randomlocation _returnvalue) (`NavigationSystemV1.K2_GetRandomLocationInNavigableRadius` (`self.K2_GetActorLocation`) (`self.Radius`) null null))
    (if _returnvalue
      (`|SpawnActorFromClass` "/Game/Moonshot/Loot/BP_Mineable_Rock.BP_Mineable_Rock_C" (`KismetMathLibrary.MakeTransform` (+ _randomlocation (`self.SpawnOffset`)) (`KismetMathLibrary.MakeRotator` 0.0 0.0 (`KismetMathLibrary.RandomFloatInRange` 0.0 1.0))) "AdjustIfPossibleButAlwaysSpawn" "OverrideRootScale" null null))))

(fn `UserConstructionScript`)