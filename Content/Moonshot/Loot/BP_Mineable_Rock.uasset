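; Mineable rock loot actor that can be grabbed by the player and broken into moonrock rubble.
; Interact casts the interactor to BP_PlayerCharacter and passes the hit to its GrabObjectByLocation.
; Break spawns RubbleCount BP_Moonrock actors at small random offsets around the Cube component, matching its rotation at unit scale, then destroys the rock.
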(event `/Game/Moonshot/BPI_Interactable.Interact`
  (params (Interactor :type "Actor Object Reference") (HitInfo :type "HitResult Structure"))
  (bind _asbp_player_character (cast `/Game/Moonshot/Characters/BP_PlayerCharacter` Interactor))
  (`/Game/Moonshot/Characters/BP_PlayerCharacter.GrabObjectByLocation` _asbp_player_character HitInfo))

(fn `Break`
  (params (NewParam :type Boolean))
  (for _ (range 1 (+ (`self.RubbleCount`) 1))
    (`|SpawnActorFromClass` "/Game/Moonshot/Loot/BP_Moonrock.BP_Moonrock_C" (`KismetMathLibrary.MakeTransform` (+ (* (`KismetMathLibrary.RandomUnitVector`) (`KismetMathLibrary.RandomFloatInRange` 5.0 50.0)) (.location (`SceneComponent.K2_GetComponentToWorld` (`self.Cube`)))) (.rotation (`SceneComponent.K2_GetComponentToWorld` (`self.Cube`))) (1.0 1.0 1.0)) "AdjustIfPossibleButAlwaysSpawn" "OverrideRootScale" null null))
  (`self.K2_DestroyActor`)
  (return))

(fn `UserConstructionScript`)