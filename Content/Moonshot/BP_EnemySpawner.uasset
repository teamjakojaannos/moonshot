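; Server-side enemy spawner actor that repeatedly spawns an Enemy class at its own transform plus a spawn offset.
; On BeginPlay the server starts a one-shot timer, and each spawn re-arms it with a base interval randomized by a variation range.
; Each spawned enemy with an AIC_BugAI controller receives an initial aggro location as its move-to target.
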(event `self.ReceiveBeginPlay`
  (if (`KismetSystemLibrary.IsServer`)
    (`KismetSystemLibrary.K2_SetTimerDelegate` (delegate `SpawnEnemy`) (`self.GetInterval`))))

(event `SpawnEnemy`
  (bind (_returnvalue_location _returnvalue_rotation _returnvalue_scale) (`KismetMathLibrary.BreakTransform` (`self.GetTransform`)))
  (bind _returnvalue (`|SpawnActorFromClass` (`self.Enemy`) (`KismetMathLibrary.MakeTransform` (+ _returnvalue_location (`self.SpawnOffset`)) _returnvalue_rotation _returnvalue_scale) "AdjustIfPossibleButAlwaysSpawn" "OverrideRootScale" null null))
  (`/Engine/EditorBlueprintResources/StandardMacros.IsValid` _returnvalue
    (:`Is Valid`
      (bind _asaic_bug_ai (cast `/Game/Moonshot/Characters/Alien/AIC_BugAI` (`AIBlueprintHelperLibrary.GetAIController` _returnvalue))
        (:`then`
          (`/Game/Moonshot/Characters/Alien/AIC_BugAI.SetMoveToLocationKey` _asaic_bug_ai (`self.InitialAggroLocation`)))
        (:`CastFailed`
          _)))
    (:`Is Not Valid`
      _))
  (`KismetSystemLibrary.K2_SetTimerDelegate` (delegate `SpawnEnemy`) (`self.GetInterval`)))

(fn `GetInterval`
  (returns (ReturnValue :type "Float (double-precision)"))
  (bind _intervalvariation (`self.IntervalVariation`))
  (return (+ (`self.Interval`) (`KismetMathLibrary.RandomFloatInRange` (* _intervalvariation -1.0) _intervalvariation))))

(fn `UserConstructionScript`)